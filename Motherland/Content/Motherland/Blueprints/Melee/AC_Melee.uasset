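; Melee combat component for a Character that plays combo attack montages and moves the weapon between hand slot and holster.
; Attack auto-equips, then cycles ground montages or plays a jump attack that a looping timer stops on landing.
; Montage notifies gate chaining and call TriggerSimpleHit, whose box-trace damage logic is disconnected.
; A socket sphere-trace alternative applies damage, sparks and a timed combo count, but nothing here calls it.
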(event `self.ReceiveBeginPlay`
  (bind _owner (`self.Owner`))
  (bind _ascharacter (cast `Character` (`self.GetOwner`)))
  (set `self.Owner` _ascharacter)
  (set `self.AttackMaxIndex` (- (`KismetArrayLibrary.Array_Length` (`self.AttackAnimations`)) 1))
  (bind (_righthandweaponequipslot _leftweaponholster) (message `/Game/Motherland/Blueprints/Character/BPI_CharacterACActions.GetCharacterEquipSceneComponenets` _owner))
  (set `self.CharacterRightHandEquipSlot` _righthandweaponequipslot)
  (set `self.CharacterWeaponHolster` _leftweaponholster)
  (bind _weaponactor (message `/Game/Motherland/Blueprints/Character/BPI_CharacterACActions.GetCharacterWeapon` _owner))
  (set `self.CharacterWeapon` _weaponactor))

(event `Attack`
  (if (`self.bCanAttack`)
    (if (not (`self.bIsWeaponEquipped?`))
      (`self.Equip Weapon` true))
    (set `self.bCanAttack` false)
    (if (not (`self.GetOwnerFallingState`))
      (bind _notifyname (`|PlayMontage` (`self.GetOwnerMesh`) (`|GetArrayItem` (`self.AttackAnimations`) (`self.AttackCurrentIndex`)))
        (:`then`
          (set `self.AttackCurrentIndex` (`KismetMathLibrary.SelectInt` (+ (`self.AttackCurrentIndex`) 1) 0 (< (`self.AttackCurrentIndex`) (`self.AttackMaxIndex`)))))
        (:`OnCompleted`
          (set `self.AttackCurrentIndex` 0)
          (set `self.bCanAttack` true))
        (:`OnNotifyBegin`
          (switch `name` _notifyname
            (:`Hit`
              (`self.TriggerSimpleHit`))
            (:`CanCombo`
              (set `self.bCanAttack` true))
            (:`Recovery`
              (set `self.bCanAttack` false)))))
      (else
        (bind _notifyname_2 (`|PlayMontage` (`self.GetOwnerMesh`) (`self.JumpAttackAnimMontage`))
          (:`then`
            (bind _returnvalue (`KismetSystemLibrary.K2_SetTimerDelegate` (delegate `CheckForGround`) 0.016667 true))
            (set `self.TH_GroundCheck` _returnvalue))
          (:`OnNotifyBegin`
            (switch `name` _notifyname_2
              (:`Hit`
                (`self.TriggerSimpleHit`))
              (:`CanCombo`
                (set `self.bCanAttack` true)))))))))

(event `CheckForGround`
  (if (`self.GetOwnerMovingOnGroundState`)
    (`Character.StopAnimMontage` (`self.Owner`) (`self.JumpAttackAnimMontage`))
    (set `self.bCanAttack` true)
    (`KismetSystemLibrary.K2_ClearAndInvalidateTimerHandle` (`self.TH_GroundCheck`))))

(event `IncrementCombo`
  (`/Engine/EditorBlueprintResources/StandardMacros.IncrementInt` (`self.ComboCount`)
    (:`  `
      (`KismetSystemLibrary.RetriggerableDelay` 2.0)
      (set `self.ComboCount` 0))))

(event `Equip Weapon`
  (params (`bIsWeaponEquippedByChar?` :type Boolean))
  (bind _characterweapon (`self.CharacterWeapon`))
  (bind _output_get (set `self.bIsWeaponEquipped?` `bIsWeaponEquippedByChar?`))
  (if _output_get
    (`|PlayMontage` (`self.GetOwnerMesh`) (`self.EquipWeaponAnimation`) 1.3
      (:`then`
        (`KismetSystemLibrary.Delay` 0.4)
        (`SceneComponent.K2_AttachToComponent` _characterweapon (`self.CharacterRightHandEquipSlot`) "None" "KeepWorld" "KeepWorld" "KeepWorld" true)))
    (else
      (`|PlayMontage` (`self.GetOwnerMesh`) (`self.EquipWeaponAnimation`) 1.3
        (:`then`
          (`KismetSystemLibrary.Delay` 0.4)
          (`SceneComponent.K2_AttachToComponent` _characterweapon (`self.CharacterWeaponHolster`) "None" "KeepWorld" "KeepWorld" "KeepWorld" true)))))
  (`KismetSystemLibrary.MoveComponentTo` _characterweapon))

(fn `GetCharacterEquipSceneComponenets`
  (returns (RightHandWeaponEquipSlot :type "SceneComponent Object Reference") (LeftWeaponHolster :type "SceneComponent Object Reference"))
  (return null null))

(fn `GetCharacterWeapon`
  (returns (WeaponActor :type "ChildActorComponent Object Reference"))
  (return null))

(fn `TriggerComplexHit`
  (bind _mesh (`Character.Mesh` (`self.Owner`)))
  (bind (_outhit _returnvalue) (`KismetSystemLibrary.SphereTraceSingleForObjects` (`SceneComponent.GetSocketLocation` _mesh "MeleeSocketStart") (`SceneComponent.GetSocketLocation` _mesh "MeleeSocketEnd") 30.0 (`|MakeArray` "ObjectTypeQuery3" :!type "EObjectTypeQuery Enum") true))
  (if _returnvalue
    (bind (_bblockinghit _binitialoverlap _time _distance _location _impactpoint _normal _impactnormal _physmat _hitactor) (`GameplayStatics.BreakHitResult` _outhit))
    (if (`Actor.bCanBeDamaged` _hitactor)
      (`GameplayStatics.ApplyDamage` _hitactor 5.0 null null "/Script/Engine.DamageType")
      (`GameplayStatics.SpawnEmitterAtLocation` "/Game/InfinityBladeEffects/Effects/FX_Combat_Base/Impact/P_ImpactSpark.P_ImpactSpark" _impactpoint)
      (`self.IncrementCombo`))))

(fn `TriggerSimpleHit`)