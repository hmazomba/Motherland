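; BP_WeatherMan is a weather actor that runs one timed rain shower shortly after play begins, then stops it.
; Toggle events switch the rain effect and sound, set the wetness change direction, and randomize or clear water ripples.
; Tick adds that rate to a wetness level each frame, driving materials through MP_GlobalParams.
; The out-of-range check re-enables tick instead of disabling it, so wetness is never clamped.
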(event `self.ReceiveBeginPlay`
  (`KismetSystemLibrary.Delay` 5.0)
  (`self.ToggleRain` true)
  (`self.ToggleRainScreenEffect` true)
  (`KismetSystemLibrary.Delay` 30.0)
  (`self.ToggleRain` false)
  (`self.ToggleRainScreenEffect` false))

(event `self.ReceiveTick`
  (params (DeltaSeconds :type "Float (single-precision)"))
  (bind _amountofrain (`self.AmountOfRain`))
  (`self.UpdateAmountOfRain`)
  (if (or (> _amountofrain 1.0) (< _amountofrain 0.0))
    (`self.SetActorTickEnabled` true)))

(event `ToggleRain`
  (params (`bIsEnabled?` :type Boolean))
  (if `bIsEnabled?`
    (`ActorComponent.SetActive` (`self.Rain`) true false)
    (`AudioComponent.Play` (`self.RainSound`) 0.0)
    (set `self.RateOfChange` 0.1)
    (`self.SetActorTickEnabled` true)
    (else
      (`ActorComponent.SetActive` (`self.Rain`) false false)
      (`AudioComponent.Stop` (`self.RainSound`))
      (set `self.RateOfChange` -0.1)
      (`self.SetActorTickEnabled` true))))

(event `ToggleRainScreenEffect`
  (params (`bIsEnabled?` :type Boolean))
  (if `bIsEnabled?`
    (`KismetMaterialLibrary.SetScalarParameterValue` "/Game/Motherland/Materials/Landscape/MP_GlobalParams.MP_GlobalParams" "WaterRippleEffect" (`KismetMathLibrary.RandomFloatInRange` 0.09 0.4))
    (else
      (`KismetMaterialLibrary.SetScalarParameterValue` "/Game/Motherland/Materials/Landscape/MP_GlobalParams.MP_GlobalParams" "WaterRippleEffect"))))

(fn `UserConstructionScript`)