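; AI controller that makes its controlled NPC pawn wander endlessly between random reachable points.
; On BeginPlay it picks a point around the pawn, starts a move to a random spot near it, and randomly toggles running through a message to the pawn.
; Each successful move restarts the cycle from the new position, while a failed one retries near the same target after a delay.
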(event `self.ReceiveBeginPlay`
  (bind _returnvalue (`self.K2_GetPawn`))
  (bind _characterpawn (`self.CharacterPawn`))
  (set `self.CharacterPawn` _returnvalue)
  (`self.GoToLocation` (`NavigationSystemV1.K2_GetRandomReachablePointInRadius` (`self.K2_GetActorLocation` _returnvalue) 2000.0 null null) :!label _label)
  (if (`KismetMathLibrary.RandomBool`)
    (message `/Game/Motherland/Blueprints/Character/BPI_CharacterActions.ToggleRun` _characterpawn true)
    (else
      (message `/Game/Motherland/Blueprints/Character/BPI_CharacterActions.ToggleRun` _characterpawn false))))

(event `self.GoToLocation`
  (params (TargetLocation :type "Vector Structure"))
  ;[0 1 0.625] Loop until you reach random point in radius
  (`|AIMoveTo` null (`NavigationSystemV1.K2_GetRandomReachablePointInRadius` TargetLocation 500.0 null null) null 200.0 :!label _label_2
    (:`OnSuccess`
      (goto _label))
    (:`OnFail`
      (`KismetSystemLibrary.Delay` 5.0)
      (goto _label_2))))

(fn `UserConstructionScript`)